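; Smart machine Blueprint that simulates a factory device over MQTT, reporting an on/off state and a randomised RPM.
; On BeginPlay it connects to a hard-coded broker and publishes JSON telemetry on a looping timer.
; It subscribes to that same per-DeviceID topic, setting IsOn from incoming messages, its own included, via substring parsing.
; RPM approximates a Gaussian by summing three random floats and is independent of IsOn.
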(event Custom|OnMessageCallback
  (params (message :type Mqtt%20Message%20Structure))
  (bind (_message _messagebuffer _topic _retain _qos) (Utilities|Struct|BreakMqttMessage message))
  (Development|PrintString (Utilities|String|Append "Message: " _message " Topic: " _topic " Retain: " (Utilities|String|ToString(Boolean) _retain) " QOS: " (Utilities|String|ToString(Integer) _qos)) true true "(R=0.327744,G=1.000000,B=0.139947,A=1.000000)" 1e+01)
  (bind _ison (CallFunction|ParseIson _message))
  (Variables|Default|SetIs_On _ison))

(event Custom|SendTelemetry
  (bind _rnd (CallFunction|GetGaussian 3.5e+03 2.5e+03))
  (Class|MqttClientInterface|Publish (Variables|Default|GetMyMqttClient) (Utilities|Struct|MakeMqttMessage (Utilities|String|Append "{" (Utilities|String|ToString(Text) (Utilities|Text|FormatText "\"is_on\": {is_on_val}, \"rpm\": {rpm_val}" (Variables|Default|GetIs_On) (Math|Float|Truncate _rnd))) "}") 0 (Utilities|String|ToString(Text) (Utilities|Text|FormatText "factory/data/{DeviceID}" (Variables|Default|GetDeviceID))))))

(event Custom|OnErrorCallback
  (params (code :type Integer) (message :type String))
  (Utilities|String|LogString (Utilities|String|ToString(Text) (Utilities|Text|ToText(String) (Utilities|String|Append "Error - Code: " (Utilities|String|ToString(Integer) code) " Message: " message)))))

(event EventBeginPlay
  (bind _returnvalue (Class|MqttUtilitiesBPL|CreateMqttClient (Utilities|Struct|MakeMqttClientConfig "192.168.0.101" 1883 (Utilities|String|Append (Variables|Default|GetDeviceID) "1") -1)))
  (bind _output_get (Variables|Default|SetMyMqttClient _returnvalue))
  (Class|MqttClientInterface|Connect _output_get (Utilities|Struct|MakeMqttConnectionData "virtplc" "virtplc123") (delegate Custom|SendTelemetry))
  (Class|MqttClientInterface|Subscribe _output_get (Utilities|String|ToString(Text) (Utilities|Text|FormatText "factory/data/{DeviceID}" (Variables|Default|GetDeviceID))))
  (Class|MqttClientInterface|SetonMessageHandler _output_get (delegate Custom|OnMessageCallback))
  (Utilities|Time|SetTimerbyEvent (delegate Custom|SendTelemetry) 0.3 true)
  (Class|MqttClientInterface|SetonErrorHandler (Variables|Default|GetMyMqttClient) (delegate Custom|OnErrorCallback)))

(event Collision|EventActorBeginOverlap
  (params (OtherActor :type Actor%20Object%20Reference)))

(event EventTick
  (params (DeltaSeconds :type Float%20%28single-precision%29)))

(fn ConstructionScript)

(fn ParseIson
  (params (JsonString :type String))
  (Variables|Default|SetValueString (Utilities|String|RightChop (Utilities|String|RightChop JsonString (Utilities|String|FindSubstring JsonString "\"is_on\":")) 8))
  (if (Utilities|String|Contains (Variables|Default|GetValueString) "true")
    (return true)
    (elif (Utilities|String|Contains (Variables|Default|GetValueString) "false")
      (return false)
      (else
        (Utilities|String|LogString "Bad Message format good is \"is_on\":true|false ")))))

(fn GetGaussian
  (params (mean :type Float%20%28double-precision%29) (std :type Float%20%28double-precision%29))
  (return (+ (* (- (+ (Math|Random|RandomFloat) (Math|Random|RandomFloat) (Math|Random|RandomFloat)) 1.5) std) mean)))