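; Pick-and-place machine that populates a PCB in a simulated production line and reports the operation through start, data-collection and complete calls.
; StartProcessCompPlace builds JSON messages by string-splitting OpDetails, with random X/Y positions as logged parameters.
; Delay-timed events chain chip, capacitor, resistor, coil and connector placement, using timelines to move the gantry and picker.
; Each carries a temporary mesh, adds one to the PCB and appends the part to its Tags[3].
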(event Custom|Place%20Coil
  (bind _coil (Variables|Default|GetCoil))
  (bind _coil_loc (Variables|Default|GetCoil%20Loc))
  (bind (_x _y _z) (Math|Vector|BreakVector _coil_loc))
  (bind _relativelocation (Variables|/Script/Engine.SceneComponent|GetRelativeLocation _coil))
  ;[1 1 1] Component Placing
  (CallFunction|PickComponent _relativelocation)
  (Utilities|FlowControl|Delay 1.1)
  (CallFunction|PickDown)
  (Utilities|FlowControl|Delay 0.6)
  (bind _returnvalue (AddComponent|AddStaticMeshComponent false (Math|Transform|MakeTransform (- _relativelocation "0.000000,0.000000,2.000000") "0.000000,90.000000,0.000000" "1.000000,1.000000,1.000000")))
  (Transformation|AttachComponentToComponent _returnvalue (Variables|Default|GetEnd%20Picker) "None" "KeepWorld" "KeepWorld" "KeepWorld" true)
  (Utilities|FlowControl|Delay 0.1)
  (CallFunction|PickUp)
  (Utilities|FlowControl|Delay 0.6)
  (CallFunction|PlaceComponent (- (Math|Vector|MakeVector (* _y -1.0) (* _x 1.0) _z) "0.000000,6.000000,0.000000") _relativelocation)
  (Utilities|FlowControl|Delay 1.1)
  (CallFunction|PlaceDown)
  (Utilities|FlowControl|Delay 0.7)
  (Components|DestroyComponent _returnvalue)
  (AddComponent|AddStaticMeshComponent (stale Custom|Start%20Process%20Comp%20Place PCB) false (Math|Transform|MakeTransform (- (Variables|Default|GetCoil%20Loc) "0.000000,0.000000,88.000000") "0, 0, 0" "1.000000,1.000000,1.000000"))
  (CallFunction|PlaceUp)
  (Utilities|FlowControl|Delay 1.0)
  (Utilities|Array|SetArrayElem (Variables|/Script/Engine.Actor|GetTags (stale Custom|Start%20Process%20Comp%20Place PCB)) 3 (Utilities|String|StringToName (Utilities|String|Append (Utilities|String|ToString(Name) (Utilities|Array|Get(acopy) (Variables|/Script/Engine.Actor|GetTags (stale Custom|Start%20Process%20Comp%20Place PCB)) 3)) "<br>1pcs " "Coil")))
  (CallFunction|PlaceConnector))

(event Custom|Place%20Chip
  (bind _chip_loc (Variables|Default|GetChip%20Loc))
  (bind _chip (Variables|Default|GetChip))
  (bind (_x _y _z) (Math|Vector|BreakVector _chip_loc))
  (bind _relativelocation (Variables|/Script/Engine.SceneComponent|GetRelativeLocation _chip))
  ;[1 1 1] Component Placing
  (CallFunction|PickComponent _relativelocation)
  (Utilities|FlowControl|Delay 1.1)
  (CallFunction|PickDown)
  (Utilities|FlowControl|Delay 0.6)
  (bind _returnvalue (AddComponent|AddStaticMeshComponent false (Math|Transform|MakeTransform _relativelocation "0.000000,90.000000,0.000000" "1.000000,1.000000,1.000000")))
  (Transformation|AttachComponentToComponent _returnvalue (Variables|Default|GetEnd%20Picker) "None" "KeepWorld" "KeepWorld" "KeepWorld" true)
  (Utilities|FlowControl|Delay 0.1)
  (CallFunction|PickUp)
  (Utilities|FlowControl|Delay 0.6)
  (CallFunction|PlaceComponent (- (Math|Vector|MakeVector (* _y -1.0) (* _x 1.0) _z) "0.000000,6.000000,0.000000") _relativelocation)
  (Utilities|FlowControl|Delay 1.1)
  (CallFunction|PlaceDown)
  (Utilities|FlowControl|Delay 0.7)
  (Components|DestroyComponent _returnvalue)
  (AddComponent|AddStaticMeshComponent (stale Custom|Start%20Process%20Comp%20Place PCB) false (Math|Transform|MakeTransform (- (Variables|Default|GetChip%20Loc) "0.000000,0.000000,88.000000") "0, 0, 0" "1.000000,1.000000,1.000000"))
  (CallFunction|PlaceUp)
  (Utilities|FlowControl|Delay 1.0)
  (Utilities|Array|SetArrayElem (Variables|/Script/Engine.Actor|GetTags (stale Custom|Start%20Process%20Comp%20Place PCB)) 3 (Utilities|String|StringToName (Utilities|String|Append (Utilities|String|ToString(Name) (Utilities|Array|Get(acopy) (Variables|/Script/Engine.Actor|GetTags (stale Custom|Start%20Process%20Comp%20Place PCB)) 3)) "<br>1pcs " "Chip")))
  (CallFunction|PlaceCapacitor))

(event Custom|Pick%20down
  ;[1 1 1] Actions
  (bind _newtrack_0 (Timeline|Timeline_Pick PlayFromStart)
    (:Update
      (Transformation|SetRelativeLocation (Variables|Default|GetEnd%20Picker) (Math|Vector|MakeVector 0.0 0.0 (Math|Float|Lerp 0.0 -1.0 _newtrack_0)) false false))))

(event Custom|Place%20down
  ;[1 1 1] Actions
  (bind _newtrack_0 (Timeline|Timeline_Place PlayFromStart)
    (:Update
      (Transformation|SetRelativeLocation (Variables|Default|GetEnd%20Picker) (Math|Vector|MakeVector 0.0 0.0 (Math|Float|Lerp 0.0 -6.0 _newtrack_0)) false false))))

(event Custom|Pick%20up
  ;[1 1 1] Actions
  (bind _newtrack_0 (Timeline|Timeline_Pick ReverseFromEnd)
    (:Update
      (Transformation|SetRelativeLocation (Variables|Default|GetEnd%20Picker) (Math|Vector|MakeVector 0.0 0.0 (Math|Float|Lerp 0.0 -1.0 _newtrack_0)) false false))))

(event Custom|Place%20up
  ;[1 1 1] Actions
  (bind _newtrack_0 (Timeline|Timeline_Place ReverseFromEnd)
    (:Update
      (Transformation|SetRelativeLocation (Variables|Default|GetEnd%20Picker) (Math|Vector|MakeVector 0.0 0.0 (Math|Float|Lerp 0.0 -6.0 _newtrack_0)) false false))))

(event Custom|Pick%20Component
  (params (Component%20Tray%20Loc :type Vector))
  ;[1 1 1] Actions
  (bind _output_get (Variables|Default|SetStart%20Location "0, 0, 0"))
  (bind _newtrack_0 (Timeline|Timeline_1 PlayFromStart)
    (:Update
      (Transformation|SetRelativeLocation (Variables|Default|GetMoveX) (Math|Vector|MakeVector (.X (Math|Vector|BreakVector (Math|Vector|Lerp(Vector) _output_get Component%20Tray%20Loc _newtrack_0))) 0.6 95.88) false false)
      (Transformation|SetRelativeLocation (Variables|Default|GetMoveEnd) (Math|Vector|MakeVector 0.0 (.Y (Math|Vector|BreakVector (Math|Vector|Lerp(Vector) _output_get Component%20Tray%20Loc _newtrack_0))) 0.0) false false))))

(event Custom|Start%20Process%20Comp%20Place
  (params (PCB :type Actor%20Object%20Reference) (SFC :type String) (Plant :type String) (OpDetails :type String))
  ;[1 1 1] Component Placing
  (Variables|Default|SetPosX (Math|Random|RandomIntegerinRange 5 10))
  (Variables|Default|SetPosY (Math|Random|RandomIntegerinRange 5 10))
  (Utilities|SetMessages SFC Plant OpDetails)
  (Variables|Default|SetInOperation true)
  (Default|CallStartOperation)
  (CallFunction|PlaceChip))

(event Custom|Place%20Capacitor
  (bind _capacitor (Variables|Default|GetCapacitor))
  (bind _capacitor_loc (Variables|Default|GetCapacitor%20Loc))
  (bind (_x _y _z) (Math|Vector|BreakVector _capacitor_loc))
  (bind _relativelocation (Variables|/Script/Engine.SceneComponent|GetRelativeLocation _capacitor))
  ;[1 1 1] Component Placing
  (CallFunction|PickComponent _relativelocation)
  (Utilities|FlowControl|Delay 1.1)
  (CallFunction|PickDown)
  (Utilities|FlowControl|Delay 0.6)
  (bind _returnvalue (AddComponent|AddStaticMeshComponent false (Math|Transform|MakeTransform (- _relativelocation "0.000000,0.000000,2.000000") "0.000000,90.000000,0.000000" "1.000000,1.000000,1.000000")))
  (Transformation|AttachComponentToComponent _returnvalue (Variables|Default|GetEnd%20Picker) "None" "KeepWorld" "KeepWorld" "KeepWorld" true)
  (Utilities|FlowControl|Delay 0.1)
  (CallFunction|PickUp)
  (Utilities|FlowControl|Delay 0.6)
  (CallFunction|PlaceComponent (- (Math|Vector|MakeVector (* _y -1.0) (* _x 1.0) _z) "0.000000,6.000000,0.000000") _relativelocation)
  (Utilities|FlowControl|Delay 1.1)
  (CallFunction|PlaceDown)
  (Utilities|FlowControl|Delay 0.7)
  (Components|DestroyComponent _returnvalue)
  (AddComponent|AddStaticMeshComponent (stale Custom|Start%20Process%20Comp%20Place PCB) false (Math|Transform|MakeTransform (- (Variables|Default|GetCapacitor%20Loc) "0.000000,0.000000,88.000000") "0, 0, 0" "1.000000,1.000000,1.000000"))
  (CallFunction|PlaceUp)
  (Utilities|FlowControl|Delay 1.0)
  (Utilities|Array|SetArrayElem (Variables|/Script/Engine.Actor|GetTags (stale Custom|Start%20Process%20Comp%20Place PCB)) 3 (Utilities|String|StringToName (Utilities|String|Append (Utilities|String|ToString(Name) (Utilities|Array|Get(acopy) (Variables|/Script/Engine.Actor|GetTags (stale Custom|Start%20Process%20Comp%20Place PCB)) 3)) "<br>1pcs " "Capacitor")))
  (CallFunction|PlaceResistor))

(event Custom|Place%20Resistor
  (bind _resistor (Variables|Default|GetResistor))
  (bind _resistor_loc (Variables|Default|GetResistor%20Loc))
  (bind (_x _y _z) (Math|Vector|BreakVector _resistor_loc))
  (bind _relativelocation (Variables|/Script/Engine.SceneComponent|GetRelativeLocation _resistor))
  ;[1 1 1] Component Placing
  (CallFunction|PickComponent _relativelocation)
  (Utilities|FlowControl|Delay 1.1)
  (CallFunction|PickDown)
  (Utilities|FlowControl|Delay 0.6)
  (bind _returnvalue (AddComponent|AddStaticMeshComponent false (Math|Transform|MakeTransform _relativelocation "0.000000,90.000000,0.000000" "1.000000,1.000000,1.000000")))
  (Transformation|AttachComponentToComponent _returnvalue (Variables|Default|GetEnd%20Picker) "None" "KeepWorld" "KeepWorld" "KeepWorld" true)
  (Utilities|FlowControl|Delay 0.1)
  (CallFunction|PickUp)
  (Utilities|FlowControl|Delay 0.6)
  (CallFunction|PlaceComponent (- (Math|Vector|MakeVector (* _y -1.0) (* _x 1.0) _z) "0.000000,6.000000,0.000000") _relativelocation)
  (Utilities|FlowControl|Delay 1.1)
  (CallFunction|PlaceDown)
  (Utilities|FlowControl|Delay 0.7)
  (Components|DestroyComponent _returnvalue)
  (AddComponent|AddStaticMeshComponent (stale Custom|Start%20Process%20Comp%20Place PCB) false (Math|Transform|MakeTransform (- (Variables|Default|GetResistor%20Loc) "0.000000,0.000000,88.000000") "0, 0, 0" "1.000000,1.000000,1.000000"))
  (CallFunction|PlaceUp)
  (Utilities|FlowControl|Delay 1.0)
  (Utilities|Array|SetArrayElem (Variables|/Script/Engine.Actor|GetTags (stale Custom|Start%20Process%20Comp%20Place PCB)) 3 (Utilities|String|StringToName (Utilities|String|Append (Utilities|String|ToString(Name) (Utilities|Array|Get(acopy) (Variables|/Script/Engine.Actor|GetTags (stale Custom|Start%20Process%20Comp%20Place PCB)) 3)) "<br>1pcs " "Resistor")))
  (CallFunction|PlaceCoil))

(event Custom|Place%20Connector
  (bind _connector (Variables|Default|GetConnector))
  (bind _connector_loc (Variables|Default|GetConnector%20Loc))
  (bind (_x _y _z) (Math|Vector|BreakVector _connector_loc))
  (bind _relativelocation (Variables|/Script/Engine.SceneComponent|GetRelativeLocation _connector))
  ;[1 1 1] Component Placing
  (CallFunction|PickComponent _relativelocation)
  (Utilities|FlowControl|Delay 1.1)
  (CallFunction|PickDown)
  (Utilities|FlowControl|Delay 0.6)
  (bind _returnvalue (AddComponent|AddStaticMeshComponent false (Math|Transform|MakeTransform _relativelocation "0.000000,90.000000,0.000000" "1.000000,1.000000,1.000000")))
  (Transformation|AttachComponentToComponent _returnvalue (Variables|Default|GetEnd%20Picker) "None" "KeepWorld" "KeepWorld" "KeepWorld" true)
  (Utilities|FlowControl|Delay 0.1)
  (CallFunction|PickUp)
  (Utilities|FlowControl|Delay 0.6)
  (CallFunction|PlaceComponent (- (Math|Vector|MakeVector (* _y -1.0) (* _x 1.0) _z) "0.000000,6.000000,0.000000") _relativelocation)
  (Utilities|FlowControl|Delay 1.1)
  (CallFunction|PlaceDown)
  (Utilities|FlowControl|Delay 0.7)
  (Components|DestroyComponent _returnvalue)
  (AddComponent|AddStaticMeshComponent (stale Custom|Start%20Process%20Comp%20Place PCB) false (Math|Transform|MakeTransform (- (Variables|Default|GetConnector%20Loc) "0.000000,0.000000,88.000000") "0, 0, 0" "1.000000,1.000000,1.000000"))
  (CallFunction|PlaceUp)
  (Default|CallDCLog)
  (Utilities|FlowControl|Delay 1.0)
  (Utilities|Array|SetArrayElem (Variables|/Script/Engine.Actor|GetTags (stale Custom|Start%20Process%20Comp%20Place PCB)) 3 (Utilities|String|StringToName (Utilities|String|Append (Utilities|String|ToString(Name) (Utilities|Array|Get(acopy) (Variables|/Script/Engine.Actor|GetTags (stale Custom|Start%20Process%20Comp%20Place PCB)) 3)) "<br>1pcs " "Connector")))
  (Variables|Default|SetInOperation false)
  (Default|CallCompleteOperation))

(event Custom|Place%20Component
  (params (Component%20Board%20Loc :type Vector) (Component%20Tray%20Loc :type Vector))
  ;[1 1 1] Actions
  (Variables|Default|SetStart%20Location "0, 0, 0")
  (bind _newtrack_0 (Timeline|Timeline_2 PlayFromStart)
    (:Update
      (Transformation|SetRelativeLocation (Variables|Default|GetMoveX) (Math|Vector|MakeVector (.X (Math|Vector|BreakVector (Math|Vector|Lerp(Vector) Component%20Tray%20Loc Component%20Board%20Loc _newtrack_0))) 0.6 95.88) false false)
      (Transformation|SetRelativeLocation (Variables|Default|GetMoveEnd) (Math|Vector|MakeVector 0.0 (.Y (Math|Vector|BreakVector (Math|Vector|Lerp(Vector) Component%20Tray%20Loc Component%20Board%20Loc _newtrack_0))) 0.0) false false))))

(event EventBeginPlay)

(fn ConstructionScript)