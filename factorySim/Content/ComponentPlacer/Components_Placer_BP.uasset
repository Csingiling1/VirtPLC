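; Virtual factory pick-and-place machine that mounts chip, capacitor, resistor, coil and connector onto a PCB.
; A looping timer starts placement and publishes MQTT status while IsOn, which is parsed from messages on that same topic.
; Chained events animate gantry and picker via timelines and delays, adding meshes and tag text to the PCB.
; SetMessages string-builds start, completion and data-collection JSON with random X/Y readings; dispatchers signal each stage.
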(event Custom|CustomEvent_2
  (params (message :type Mqtt%20Message%20Structure))
  (bind (_message _messagebuffer _topic _retain _qos) (Utilities|Struct|BreakMqttMessage message))
  (Development|PrintString (Utilities|String|Append "Message: " _message " Topic: " _topic " Retain: " (Utilities|String|ToString(Boolean) _retain) " QOS: " (Utilities|String|ToString(Integer) _qos)) true true "(R=0.327744,G=1.000000,B=0.139947,A=1.000000)" 1e+01)
  (bind _ison (CallFunction|ParseIson _message))
  (Variables|Default|SetIs_on _ison))

(event Custom|CustomEvent_1
  (if (Variables|Default|GetIs_on)
    (CallFunction|StartProcessCompPlace)
    (Class|MqttClientInterface|Publish (Variables|Default|GetMyMqttClient_0) (Utilities|Struct|MakeMqttMessage (Utilities|String|Append "{" (Utilities|String|ToString(Text) (Utilities|Text|FormatText "\"is_on\": {is_on_val}, \"posX\": {posX}, \"posY\": {posY}. \"In_operation\": {is_busy}" (Variables|Default|GetIs_on) (Variables|Default|GetPosX) (Variables|Default|GetPosY) (Variables|Default|GetInOperation))) "}") 0 (Utilities|String|ToString(Text) (Utilities|Text|FormatText "factory/data/{DeviceID}" (Utilities|String|Append (Variables|Default|GetDeviceID_0) "1")))))
    (else
      (Variables|Default|SetInOperation false)
      (Default|CallCompleteOperation))))

(event Custom|Pick%20down
  ;[1 1 1] Actions
  (bind _newtrack_0 (Timeline|Timeline_Pick PlayFromStart)
    (:Update
      (Transformation|SetRelativeLocation (Variables|Default|GetEnd%20Picker) (Math|Vector|MakeVector 0.0 0.0 (Math|Float|Lerp 0.0 -1.0 _newtrack_0)) false false))))

(event Custom|Place%20down
  ;[1 1 1] Actions
  (bind _newtrack_0 (Timeline|Timeline_Place PlayFromStart)
    (:Update
      (Transformation|SetRelativeLocation (Variables|Default|GetEnd%20Picker) (Math|Vector|MakeVector 0.0 0.0 (Math|Float|Lerp 0.0 -6.0 _newtrack_0)) false false))))

(event Custom|Pick%20up
  ;[1 1 1] Actions
  (bind _newtrack_0 (Timeline|Timeline_Pick ReverseFromEnd)
    (:Update
      (Transformation|SetRelativeLocation (Variables|Default|GetEnd%20Picker) (Math|Vector|MakeVector 0.0 0.0 (Math|Float|Lerp 0.0 -1.0 _newtrack_0)) false false))))

(event Custom|Place%20up
  ;[1 1 1] Actions
  (bind _newtrack_0 (Timeline|Timeline_Place ReverseFromEnd)
    (:Update
      (Transformation|SetRelativeLocation (Variables|Default|GetEnd%20Picker) (Math|Vector|MakeVector 0.0 0.0 (Math|Float|Lerp 0.0 -6.0 _newtrack_0)) false false))))

(event Custom|Pick%20Component
  (params (Component%20Tray%20Loc :type Vector))
  ;[1 1 1] Actions
  (bind _output_get (Variables|Default|SetStart%20Location "0, 0, 0"))
  (bind _newtrack_0 (Timeline|Timeline_1 PlayFromStart)
    (:Update
      (Transformation|SetRelativeLocation (Variables|Default|GetMoveX) (Math|Vector|MakeVector (.X (Math|Vector|BreakVector (Math|Vector|Lerp(Vector) _output_get Component%20Tray%20Loc _newtrack_0))) 0.6 95.88) false false)
      (Transformation|SetRelativeLocation (Variables|Default|GetMoveEnd) (Math|Vector|MakeVector 0.0 (.Y (Math|Vector|BreakVector (Math|Vector|Lerp(Vector) _output_get Component%20Tray%20Loc _newtrack_0))) 0.0) false false))))

(event Custom|Start%20Process%20Comp%20Place
  (params (PCB :type Actor%20Object%20Reference) (SFC :type String) (Plant :type String) (OpDetails :type String))
  ;[1 1 1] Component Placing
  (Variables|Default|SetPosX (Math|Random|RandomIntegerinRange 5 10))
  (Variables|Default|SetPosY (Math|Random|RandomIntegerinRange 5 10))
  (Utilities|SetMessages SFC Plant OpDetails)
  (Variables|Default|SetInOperation true)
  (Default|CallStartOperation)
  (CallFunction|PlaceChip))

(event Custom|Place%20Capacitor
  (bind _capacitor (Variables|Default|GetCapacitor))
  (bind _capacitor_loc (Variables|Default|GetCapacitor%20Loc))
  (bind (_x _y _z) (Math|Vector|BreakVector _capacitor_loc))
  (bind _relativelocation (Variables|/Script/Engine.SceneComponent|GetRelativeLocation _capacitor))
  ;[1 1 1] Component Placing
  (CallFunction|PickComponent _relativelocation)
  (Utilities|FlowControl|Delay 1.1)
  (CallFunction|PickDown)
  (Utilities|FlowControl|Delay 0.6)
  (bind _returnvalue (AddComponent|AddStaticMeshComponent false (Math|Transform|MakeTransform (- _relativelocation "0.000000,0.000000,2.000000") "0.000000,90.000000,0.000000" "1.000000,1.000000,1.000000")))
  (Transformation|AttachComponentToComponent _returnvalue (Variables|Default|GetEnd%20Picker) "None" "KeepWorld" "KeepWorld" "KeepWorld" true)
  (Utilities|FlowControl|Delay 0.1)
  (CallFunction|PickUp)
  (Utilities|FlowControl|Delay 0.6)
  (CallFunction|PlaceComponent (- (Math|Vector|MakeVector (* _y -1.0) (* _x 1.0) _z) "0.000000,6.000000,0.000000") _relativelocation)
  (Utilities|FlowControl|Delay 1.1)
  (CallFunction|PlaceDown)
  (Utilities|FlowControl|Delay 0.7)
  (Components|DestroyComponent _returnvalue)
  (AddComponent|AddStaticMeshComponent (stale Custom|Start%20Process%20Comp%20Place PCB) false (Math|Transform|MakeTransform (- (Variables|Default|GetCapacitor%20Loc) "0.000000,0.000000,88.000000") "0, 0, 0" "1.000000,1.000000,1.000000"))
  (CallFunction|PlaceUp)
  (Utilities|FlowControl|Delay 1.0)
  (Utilities|Array|SetArrayElem (Variables|/Script/Engine.Actor|GetTags (stale Custom|Start%20Process%20Comp%20Place PCB)) 3 (Utilities|String|StringToName (Utilities|String|Append (Utilities|String|ToString(Name) (Utilities|Array|Get(acopy) (Variables|/Script/Engine.Actor|GetTags (stale Custom|Start%20Process%20Comp%20Place PCB)) 3)) "<br>1pcs " "Capacitor")))
  (CallFunction|PlaceResistor))

(event Custom|Place%20Chip
  (bind _chip_loc (Variables|Default|GetChip%20Loc))
  (bind _chip (Variables|Default|GetChip))
  (bind (_x _y _z) (Math|Vector|BreakVector _chip_loc))
  (bind _relativelocation (Variables|/Script/Engine.SceneComponent|GetRelativeLocation _chip))
  ;[1 1 1] Component Placing
  (CallFunction|PickComponent _relativelocation)
  (Utilities|FlowControl|Delay 1.1)
  (CallFunction|PickDown)
  (Utilities|FlowControl|Delay 0.6)
  (bind _returnvalue (AddComponent|AddStaticMeshComponent false (Math|Transform|MakeTransform _relativelocation "0.000000,90.000000,0.000000" "1.000000,1.000000,1.000000")))
  (Transformation|AttachComponentToComponent _returnvalue (Variables|Default|GetEnd%20Picker) "None" "KeepWorld" "KeepWorld" "KeepWorld" true)
  (Utilities|FlowControl|Delay 0.1)
  (CallFunction|PickUp)
  (Utilities|FlowControl|Delay 0.6)
  (CallFunction|PlaceComponent (- (Math|Vector|MakeVector (* _y -1.0) (* _x 1.0) _z) "0.000000,6.000000,0.000000") _relativelocation)
  (Utilities|FlowControl|Delay 1.1)
  (CallFunction|PlaceDown)
  (Utilities|FlowControl|Delay 0.7)
  (Components|DestroyComponent _returnvalue)
  (AddComponent|AddStaticMeshComponent (stale Custom|Start%20Process%20Comp%20Place PCB) false (Math|Transform|MakeTransform (- (Variables|Default|GetChip%20Loc) "0.000000,0.000000,88.000000") "0, 0, 0" "1.000000,1.000000,1.000000"))
  (CallFunction|PlaceUp)
  (Utilities|FlowControl|Delay 1.0)
  (Utilities|Array|SetArrayElem (Variables|/Script/Engine.Actor|GetTags (stale Custom|Start%20Process%20Comp%20Place PCB)) 3 (Utilities|String|StringToName (Utilities|String|Append (Utilities|String|ToString(Name) (Utilities|Array|Get(acopy) (Variables|/Script/Engine.Actor|GetTags (stale Custom|Start%20Process%20Comp%20Place PCB)) 3)) "<br>1pcs " "Chip")))
  (CallFunction|PlaceCapacitor))

(event Custom|Place%20Resistor
  (bind _resistor (Variables|Default|GetResistor))
  (bind _resistor_loc (Variables|Default|GetResistor%20Loc))
  (bind (_x _y _z) (Math|Vector|BreakVector _resistor_loc))
  (bind _relativelocation (Variables|/Script/Engine.SceneComponent|GetRelativeLocation _resistor))
  ;[1 1 1] Component Placing
  (CallFunction|PickComponent _relativelocation)
  (Utilities|FlowControl|Delay 1.1)
  (CallFunction|PickDown)
  (Utilities|FlowControl|Delay 0.6)
  (bind _returnvalue (AddComponent|AddStaticMeshComponent false (Math|Transform|MakeTransform _relativelocation "0.000000,90.000000,0.000000" "1.000000,1.000000,1.000000")))
  (Transformation|AttachComponentToComponent _returnvalue (Variables|Default|GetEnd%20Picker) "None" "KeepWorld" "KeepWorld" "KeepWorld" true)
  (Utilities|FlowControl|Delay 0.1)
  (CallFunction|PickUp)
  (Utilities|FlowControl|Delay 0.6)
  (CallFunction|PlaceComponent (- (Math|Vector|MakeVector (* _y -1.0) (* _x 1.0) _z) "0.000000,6.000000,0.000000") _relativelocation)
  (Utilities|FlowControl|Delay 1.1)
  (CallFunction|PlaceDown)
  (Utilities|FlowControl|Delay 0.7)
  (Components|DestroyComponent _returnvalue)
  (AddComponent|AddStaticMeshComponent (stale Custom|Start%20Process%20Comp%20Place PCB) false (Math|Transform|MakeTransform (- (Variables|Default|GetResistor%20Loc) "0.000000,0.000000,88.000000") "0, 0, 0" "1.000000,1.000000,1.000000"))
  (CallFunction|PlaceUp)
  (Utilities|FlowControl|Delay 1.0)
  (Utilities|Array|SetArrayElem (Variables|/Script/Engine.Actor|GetTags (stale Custom|Start%20Process%20Comp%20Place PCB)) 3 (Utilities|String|StringToName (Utilities|String|Append (Utilities|String|ToString(Name) (Utilities|Array|Get(acopy) (Variables|/Script/Engine.Actor|GetTags (stale Custom|Start%20Process%20Comp%20Place PCB)) 3)) "<br>1pcs " "Resistor")))
  (CallFunction|PlaceCoil))

(event Custom|CustomEvent_3
  (params (code :type Integer) (message :type String))
  (Utilities|String|LogString (Utilities|String|ToString(Text) (Utilities|Text|ToText(String) (Utilities|String|Append "Error - Code: " (Utilities|String|ToString(Integer) code) " Message: " message)))))

(event Custom|Place%20Connector
  (bind _connector (Variables|Default|GetConnector))
  (bind _connector_loc (Variables|Default|GetConnector%20Loc))
  (bind (_x _y _z) (Math|Vector|BreakVector _connector_loc))
  (bind _relativelocation (Variables|/Script/Engine.SceneComponent|GetRelativeLocation _connector))
  ;[1 1 1] Component Placing
  (CallFunction|PickComponent _relativelocation)
  (Utilities|FlowControl|Delay 1.1)
  (CallFunction|PickDown)
  (Utilities|FlowControl|Delay 0.6)
  (bind _returnvalue (AddComponent|AddStaticMeshComponent false (Math|Transform|MakeTransform _relativelocation "0.000000,90.000000,0.000000" "1.000000,1.000000,1.000000")))
  (Transformation|AttachComponentToComponent _returnvalue (Variables|Default|GetEnd%20Picker) "None" "KeepWorld" "KeepWorld" "KeepWorld" true)
  (Utilities|FlowControl|Delay 0.1)
  (CallFunction|PickUp)
  (Utilities|FlowControl|Delay 0.6)
  (CallFunction|PlaceComponent (- (Math|Vector|MakeVector (* _y -1.0) (* _x 1.0) _z) "0.000000,6.000000,0.000000") _relativelocation)
  (Utilities|FlowControl|Delay 1.1)
  (CallFunction|PlaceDown)
  (Utilities|FlowControl|Delay 0.7)
  (Components|DestroyComponent _returnvalue)
  (AddComponent|AddStaticMeshComponent (stale Custom|Start%20Process%20Comp%20Place PCB) false (Math|Transform|MakeTransform (- (Variables|Default|GetConnector%20Loc) "0.000000,0.000000,88.000000") "0, 0, 0" "1.000000,1.000000,1.000000"))
  (CallFunction|PlaceUp)
  (Default|CallDCLog)
  (Utilities|FlowControl|Delay 1.0)
  (Utilities|Array|SetArrayElem (Variables|/Script/Engine.Actor|GetTags (stale Custom|Start%20Process%20Comp%20Place PCB)) 3 (Utilities|String|StringToName (Utilities|String|Append (Utilities|String|ToString(Name) (Utilities|Array|Get(acopy) (Variables|/Script/Engine.Actor|GetTags (stale Custom|Start%20Process%20Comp%20Place PCB)) 3)) "<br>1pcs " "Connector")))
  (Variables|Default|SetInOperation false)
  (Default|CallCompleteOperation))

(event Custom|Place%20Coil
  (bind _coil (Variables|Default|GetCoil))
  (bind _coil_loc (Variables|Default|GetCoil%20Loc))
  (bind (_x _y _z) (Math|Vector|BreakVector _coil_loc))
  (bind _relativelocation (Variables|/Script/Engine.SceneComponent|GetRelativeLocation _coil))
  ;[1 1 1] Component Placing
  (CallFunction|PickComponent _relativelocation)
  (Utilities|FlowControl|Delay 1.1)
  (CallFunction|PickDown)
  (Utilities|FlowControl|Delay 0.6)
  (bind _returnvalue (AddComponent|AddStaticMeshComponent false (Math|Transform|MakeTransform (- _relativelocation "0.000000,0.000000,2.000000") "0.000000,90.000000,0.000000" "1.000000,1.000000,1.000000")))
  (Transformation|AttachComponentToComponent _returnvalue (Variables|Default|GetEnd%20Picker) "None" "KeepWorld" "KeepWorld" "KeepWorld" true)
  (Utilities|FlowControl|Delay 0.1)
  (CallFunction|PickUp)
  (Utilities|FlowControl|Delay 0.6)
  (CallFunction|PlaceComponent (- (Math|Vector|MakeVector (* _y -1.0) (* _x 1.0) _z) "0.000000,6.000000,0.000000") _relativelocation)
  (Utilities|FlowControl|Delay 1.1)
  (CallFunction|PlaceDown)
  (Utilities|FlowControl|Delay 0.7)
  (Components|DestroyComponent _returnvalue)
  (AddComponent|AddStaticMeshComponent (stale Custom|Start%20Process%20Comp%20Place PCB) false (Math|Transform|MakeTransform (- (Variables|Default|GetCoil%20Loc) "0.000000,0.000000,88.000000") "0, 0, 0" "1.000000,1.000000,1.000000"))
  (CallFunction|PlaceUp)
  (Utilities|FlowControl|Delay 1.0)
  (Utilities|Array|SetArrayElem (Variables|/Script/Engine.Actor|GetTags (stale Custom|Start%20Process%20Comp%20Place PCB)) 3 (Utilities|String|StringToName (Utilities|String|Append (Utilities|String|ToString(Name) (Utilities|Array|Get(acopy) (Variables|/Script/Engine.Actor|GetTags (stale Custom|Start%20Process%20Comp%20Place PCB)) 3)) "<br>1pcs " "Coil")))
  (CallFunction|PlaceConnector))

(event Custom|Place%20Component
  (params (Component%20Board%20Loc :type Vector) (Component%20Tray%20Loc :type Vector))
  ;[1 1 1] Actions
  (Variables|Default|SetStart%20Location "0, 0, 0")
  (bind _newtrack_0 (Timeline|Timeline_2 PlayFromStart)
    (:Update
      (Transformation|SetRelativeLocation (Variables|Default|GetMoveX) (Math|Vector|MakeVector (.X (Math|Vector|BreakVector (Math|Vector|Lerp(Vector) Component%20Tray%20Loc Component%20Board%20Loc _newtrack_0))) 0.6 95.88) false false)
      (Transformation|SetRelativeLocation (Variables|Default|GetMoveEnd) (Math|Vector|MakeVector 0.0 (.Y (Math|Vector|BreakVector (Math|Vector|Lerp(Vector) Component%20Tray%20Loc Component%20Board%20Loc _newtrack_0))) 0.0) false false))))

(event Collision|EventActorBeginOverlap
  (params (OtherActor :type Actor%20Object%20Reference)))

(event EventTick
  (params (DeltaSeconds :type Float%20%28single-precision%29)))

(event EventBeginPlay
  (Collision|SetCollisionEnabled (Variables|Default|GetMoveX) "NoCollision")
  (bind _returnvalue (Class|MqttUtilitiesBPL|CreateMqttClient (Utilities|Struct|MakeMqttClientConfig "192.168.0.101" 1883 (Utilities|String|Append (Variables|Default|GetDeviceID_0) "1") -1)))
  (bind _output_get (Variables|Default|SetMyMqttClient_0 _returnvalue))
  (Class|MqttClientInterface|Connect _output_get (Utilities|Struct|MakeMqttConnectionData "virtplc" "virtplc123") (delegate Custom|CustomEvent_1))
  (Class|MqttClientInterface|Subscribe _output_get (Utilities|String|ToString(Text) (Utilities|Text|FormatText "factory/data/{DeviceID}" (Utilities|String|Append (Variables|Default|GetDeviceID_0) "1"))))
  (Class|MqttClientInterface|SetonMessageHandler _output_get (delegate Custom|CustomEvent_2))
  (Utilities|Time|SetTimerbyEvent (delegate Custom|CustomEvent_1) 0.3 true)
  (Class|MqttClientInterface|SetonErrorHandler (Variables|Default|GetMyMqttClient_0) (delegate Custom|CustomEvent_3)))

(fn ConstructionScript)

(fn ParseIson
  (params (JsonString :type String))
  (Variables|Default|SetValueString (Utilities|String|RightChop (Utilities|String|RightChop JsonString (Utilities|String|FindSubstring JsonString "\"is_on\":")) 8))
  (if (Utilities|String|Contains (Variables|Default|GetValueString) "true")
    (return true)
    (elif (Utilities|String|Contains (Variables|Default|GetValueString) "false")
      (return false)
      (else
        (Utilities|String|LogString "Bad Message format good is \"is_on\":true|false ")))))