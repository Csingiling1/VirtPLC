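; Covered conveyor Blueprint that acts as an MQTT-connected machine, publishing simulated telemetry.
; On BeginPlay it hides its 3D text, connects to a hard-coded broker and subscribes to its device topic under factory/data.
; Incoming messages are printed and parsed to set the on/off state.
; While on, a looping timer publishes that state and a Gaussian-random RPM as JSON to the same topic it subscribes to.
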(event Custom|CustomEvent_2
  (params (message :type Mqtt%20Message%20Structure))
  (bind (_message _messagebuffer _topic _retain _qos) (Utilities|Struct|BreakMqttMessage message))
  (Development|PrintString (Utilities|String|Append "Message: " _message " Topic: " _topic " Retain: " (Utilities|String|ToString(Boolean) _retain) " QOS: " (Utilities|String|ToString(Integer) _qos)) true true "(R=0.327744,G=1.000000,B=0.139947,A=1.000000)" 1e+01)
  (bind _ison (CallFunction|ParseIson _message))
  (Variables|Default|SetIs_On_0 _ison))

(event Custom|CustomEvent_1
  (if (Variables|Default|GetIs_On_0)
    (bind _rnd (CallFunction|GetGaussian 3.5e+03 2.5e+03))
    (Class|MqttClientInterface|Publish (Variables|Default|GetMyMqttClient_0) (Utilities|Struct|MakeMqttMessage (Utilities|String|Append "{" (Utilities|String|ToString(Text) (Utilities|Text|FormatText "\"is_on\": {is_on_val}, \"rpm\": {rpm_val}" (Variables|Default|GetIs_On_0) (Math|Float|Truncate _rnd))) "}") 0 (Utilities|String|ToString(Text) (Utilities|Text|FormatText "factory/data/{DeviceID}" (Utilities|String|Append (Variables|Default|GetDeviceID_0) "1")))))))

(event Custom|CustomEvent_3
  (params (code :type Integer) (message :type String))
  (Utilities|String|LogString (Utilities|String|ToString(Text) (Utilities|Text|ToText(String) (Utilities|String|Append "Error - Code: " (Utilities|String|ToString(Integer) code) " Message: " message)))))

(event Collision|EventActorBeginOverlap
  (params (OtherActor :type Actor%20Object%20Reference)))

(event EventTick
  (params (DeltaSeconds :type Float%20%28single-precision%29)))

(event EventBeginPlay
  (Rendering|SetVisibility (Variables|Default|GetText3D) false false)
  (bind _returnvalue (Class|MqttUtilitiesBPL|CreateMqttClient (Utilities|Struct|MakeMqttClientConfig "192.168.0.101" 1883 (Utilities|String|Append (Variables|Default|GetDeviceID_0) "1") -1)))
  (bind _output_get (Variables|Default|SetMyMqttClient_0 _returnvalue))
  (Class|MqttClientInterface|Connect _output_get (Utilities|Struct|MakeMqttConnectionData "virtplc" "virtplc123") (delegate Custom|CustomEvent_1))
  (Class|MqttClientInterface|Subscribe _output_get (Utilities|String|ToString(Text) (Utilities|Text|FormatText "factory/data/{DeviceID}" (Utilities|String|Append (Variables|Default|GetDeviceID_0) "1"))))
  (Class|MqttClientInterface|SetonMessageHandler _output_get (delegate Custom|CustomEvent_2))
  (Utilities|Time|SetTimerbyEvent (delegate Custom|CustomEvent_1) 0.3 true)
  (Class|MqttClientInterface|SetonErrorHandler (Variables|Default|GetMyMqttClient_0) (delegate Custom|CustomEvent_3)))

(fn ConstructionScript)